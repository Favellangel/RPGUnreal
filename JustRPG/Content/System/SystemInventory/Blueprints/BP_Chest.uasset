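; BP_Chest is an interactable chest that opens a storage inventory for the player character.
; Its range overlap toggles a prompt widget and sets or clears the character's NearbyChest reference.
; Interacting lazily spawns a BP_Storage, shows its slot widget, refreshes the inventory and freezes movement.
; Closing hides storage, restores walking and resets the DoOnce that blocks repeated opening.
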(event `self.InteractionRange.OnComponentBeginOverlap`
  (params (OverlappedComponent :type "PrimitiveComponent Object Reference") (OtherActor :type "Actor Object Reference") (OtherComp :type "PrimitiveComponent Object Reference") (OtherBodyIndex :type Integer) (bFromSweep :type Boolean) (SweepResult :type "HitResult Structure (by ref)"))
  (bind _asbp_character (cast `/Game/Character/BP_character` OtherActor))
  (`SceneComponent.SetVisibility` (`self.W_ChestTxt`) true false)
  (set `/Game/Character/BP_character.NearbyChest` self _asbp_character))

(event `self.InteractionRange.OnComponentEndOverlap`
  (params (OverlappedComponent :type "PrimitiveComponent Object Reference") (OtherActor :type "Actor Object Reference") (OtherComp :type "PrimitiveComponent Object Reference") (OtherBodyIndex :type Integer))
  (bind _asbp_character (cast `/Game/Character/BP_character` OtherActor))
  (`SceneComponent.SetVisibility` (`self.W_ChestTxt`) false false)
  (set `/Game/Character/BP_character.NearbyChest` null _asbp_character))

(event `OnInteract`
  (params (Character :type "/Game/Character/BP_character Object Reference"))
  (bind _storage (`self.Storage`))
  (bind _character (`self.Character`))
  (bind _inventoryref (`/Game/Character/BP_character.InventoryRef` _character))
  (bind _charactermovement (`Character.CharacterMovement` _character))
  (`/Engine/EditorBlueprintResources/StandardMacros.DoOnce` false :!label _label
    (:`Completed`
      (set `self.Character` Character)
      (`/Engine/EditorBlueprintResources/StandardMacros.IsValid` (`self.Storage`)
        (:`Is Valid`
          _)
        (:`Is Not Valid`
          (bind _returnvalue (`|SpawnActorFromClass` "/Game/System/SystemInventory/Blueprints/BP_Storage.BP_Storage_C" (`KismetMathLibrary.MakeTransform` (0.0 0.0 0.0)) "Undefined" "OverrideRootScale" null (`self.AmountOfSlots`) (`self.Character`) (`self.SLotsPerFlow`) self null))
          (set `self.Storage` _returnvalue)))
      (`/Game/System/SystemInventory/Widgets/Storage/WB_Storage.Generate Slot Widget` (`/Game/System/SystemInventory/Blueprints/BP_Storage.WB Storage` _storage) _storage)
      (`/Game/System/SystemInventory/Blueprints/BP_Storage.VisibilityStorage` _storage true)
      (`/Game/System/SystemInventory/Blueprints/BP_Inventory.HideInventory` _inventoryref)
      (`/Game/System/SystemInventory/Blueprints/BP_Inventory.ShowInventory` _inventoryref)
      (`CharacterMovementComponent.DisableMovement` _charactermovement)
      (`MovementComponent.StopMovementImmediately` _charactermovement))))

(event `OnStorageClosed`
  (bind _character (`self.Character`))
  (bind _inventoryref (`/Game/Character/BP_character.InventoryRef` _character))
  (`/Game/System/SystemInventory/Blueprints/BP_Storage.VisibilityStorage` (`self.Storage`) false)
  (`CharacterMovementComponent.SetMovementMode` (`Character.CharacterMovement` _character) "MOVE_Walking" 0)
  (if (`/Game/System/SystemInventory/Blueprints/BP_Inventory.IsVisible?` _inventoryref)
    (`/Game/System/SystemInventory/Blueprints/BP_Inventory.HideInventory` _inventoryref)
    (`/Game/System/SystemInventory/Blueprints/BP_Inventory.ShowInventory` _inventoryref)
    (goto _label :!via `Reset`)
    (else
      (goto _label :!via `Reset`))))

(fn `UserConstructionScript`)