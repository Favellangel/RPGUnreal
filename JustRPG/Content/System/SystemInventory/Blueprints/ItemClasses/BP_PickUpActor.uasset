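; BP_PickUpActor is a world pickup for an item class and amount, taking its mesh, scale and interaction radius from the item's defaults.
; Sphere overlaps maintain the character's NearbyPickUpActors queue, showing the name and amount widget only on the first entry.
; OnPickUp credits gold directly or adds other items to the inventory, keeping any remainder in the world and logging some outcomes in LootedPickUps.
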(event `self.ReceiveTick`
  (params (DeltaSeconds :type "Float (single-precision)")))

(event `OnPickUp`
  (params (Character :type "/Game/Character/BP_character Object Reference"))
  (bind _inventoryref (`/Game/Character/BP_character.InventoryRef` Character))
  (bind _nearbypickupactors (`/Game/Character/BP_character.NearbyPickUpActors` Character))
  (bind _output (`|GetArrayItem` _nearbypickupactors))
  (if (!= (`self.Item Class`) "/Game/System/SystemInventory/Blueprints/ItemClasses/items/Gold.Gold_C")
    (`/Engine/EditorBlueprintResources/StandardMacros.IsValid` _inventoryref
      (:`Is Valid`
        (bind (_success_ _rest) (`/Game/System/SystemInventory/Blueprints/BP_Inventory.Add Item` _inventoryref (`self.Item Class`) (`self.Amount`) true))
        (if _success_
          (if (> _rest 0)
            (set `self.Amount` _rest)
            (`self.UpdateText`)
            (`KismetArrayLibrary.Array_Add` (`/Game/System/SystemInventory/Blueprints/BP_Inventory.LootedPickUps` (`/Game/Character/BP_character.InventoryRef` Character)) (make `/Game/System/SystemInventory/Blueprints/Structures/S_Inventory` (`self.ID`) (`self.Amount`)))
            (else
              (`self.K2_DestroyActor`)))
          (else
            (`KismetArrayLibrary.Array_Add` (`/Game/System/SystemInventory/Blueprints/BP_Inventory.LootedPickUps` _inventoryref) (make `/Game/System/SystemInventory/Blueprints/Structures/S_Inventory` (`self.ID`)))
            (`KismetArrayLibrary.Array_RemoveItem` _nearbypickupactors self)
            (`/Engine/EditorBlueprintResources/StandardMacros.IsValid` _output
              (:`Is Valid`
                (`SceneComponent.SetVisibility` (`/Game/System/SystemInventory/Blueprints/ItemClasses/BP_PickUpActor.W_PickUpText` _output) true false)
                (`self.K2_DestroyActor`))
              (:`Is Not Valid`
                (`self.K2_DestroyActor`)))))))
    (else
      (`/Game/Character/BP_character.IncreaseGold` Character (`self.Amount`))
      (`self.K2_DestroyActor`))))

(event `self.ReceiveBeginPlay`
  (`self.UpdateText`))

(event `self.Sphere.OnComponentBeginOverlap`
  (params (OverlappedComponent :type "PrimitiveComponent Object Reference") (OtherActor :type "Actor Object Reference") (OtherComp :type "PrimitiveComponent Object Reference") (OtherBodyIndex :type Integer) (bFromSweep :type Boolean) (SweepResult :type "HitResult Structure (by ref)"))
  (bind _asbp_character (cast `/Game/Character/BP_character` OtherActor))
  (bind _nearbypickupactors (`/Game/Character/BP_character.NearbyPickUpActors` _asbp_character))
  (if (> (`KismetArrayLibrary.Array_Length` _nearbypickupactors) 0)
    (`KismetArrayLibrary.Array_Add` _nearbypickupactors self)
    (else
      (`SceneComponent.SetVisibility` (`self.W_PickUpText`) true false)
      (`KismetArrayLibrary.Array_Add` _nearbypickupactors self))))

(event `self.Sphere.OnComponentEndOverlap`
  (params (OverlappedComponent :type "PrimitiveComponent Object Reference") (OtherActor :type "Actor Object Reference") (OtherComp :type "PrimitiveComponent Object Reference") (OtherBodyIndex :type Integer))
  (bind _asbp_character (cast `/Game/Character/BP_character` OtherActor))
  (bind _nearbypickupactors (`/Game/Character/BP_character.NearbyPickUpActors` _asbp_character))
  (bind _output (`|GetArrayItem` _nearbypickupactors))
  (if (and (`KismetSystemLibrary.IsValid` _output) (== _output self))
    (`SceneComponent.SetVisibility` (`self.W_PickUpText`) false false)
    (`KismetArrayLibrary.Array_RemoveItem` _nearbypickupactors self)
    (bind _output_2 (`|GetArrayItem` _nearbypickupactors))
    (`/Engine/EditorBlueprintResources/StandardMacros.IsValid` _output_2
      (:`Is Valid`
        (`SceneComponent.SetVisibility` (`/Game/System/SystemInventory/Blueprints/ItemClasses/BP_PickUpActor.W_PickUpText` _output_2) true false)))
    (else
      (`KismetArrayLibrary.Array_RemoveItem` _nearbypickupactors self))))

(fn `On Unhovered`
  (`PrimitiveComponent.SetMaterial` (`self.StaticMesh`) 0 (`self.OriginalMaterial`)))

(fn `UpdateText`
  (bind _aswb_pick_up_text (cast `/Game/System/SystemInventory/Widgets/WB_PickUpText` (`WidgetComponent.GetUserWidgetObject` (`self.W_PickUpText`)))
    (:`then`
      (`TextBlock.SetText` (`/Game/System/SystemInventory/Widgets/WB_PickUpText.NameTxt` _aswb_pick_up_text) (`|FormatText` "{Name} ({Amount})" (`.Name_2_108572924C75F70E67BBC4885E69F079` (break `/Game/System/SystemInventory/Blueprints/Structures/S_ItemInfo` (defaults `Object` (`self.Item Class`)))) (`KismetTextLibrary.Conv_IntToText` (`self.Amount`)))))
    (:`CastFailed`
      _))
  (return))

(fn `UserConstructionScript`
  (bind _item_class (`self.Item Class`))
  (bind _staticmesh (`self.StaticMesh`))
  (bind (_name _description _icon _canbeused _usetext _canbestacked _category _pickupmesh _meshscale _interactradius) (break `/Game/System/SystemInventory/Blueprints/Structures/S_ItemInfo` (defaults `Object` _item_class)))
  (if (`KismetSystemLibrary.IsValidClass` _item_class)
    (`StaticMeshComponent.SetStaticMesh` _staticmesh _pickupmesh)
    (set `self.OriginalMaterial` (`PrimitiveComponent.GetMaterial` _staticmesh 0))
    (`SceneComponent.SetRelativeScale3D` _staticmesh _meshscale)
    (`SphereComponent.SetSphereRadius` (`self.Sphere`) _interactradius false)))