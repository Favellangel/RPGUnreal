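; BP_Storage is a slot-based item storage that works alongside the player's inventory, with its own widget it can show or hide.
; Slot functions add, remove, swap, merge and accept items moved from inventory, refreshing the affected widget slots.
; AddItem recursively fills partial stacks, then empty slots, reporting any remainder.
; Dropped items spawn as BP_PickUpActor: line traces rotate the character's capsule seeking clear space, falling back to its location.
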(event `self.ReceiveBeginPlay`
  (set `self.WB Storage` (`/Game/Widgets/WB_MainWidget.WB_Storage` (`/Game/System/SystemInventory/Blueprints/BP_Inventory.MainWidget` (`/Game/Character/BP_character.InventoryRef` (`self.TopDownCharRef`)))))
  (`KismetArrayLibrary.Array_Resize` (`self.Slots`) (`self.AmountOfSlots`)))

(event `UpdateSlotsAtIndex`
  (params (Index :type Integer))
  (`/Game/System/SystemInventory/Widgets/Storage/WB_StorageSlot.UpdateSlot` (`|GetArrayItem` (`/Game/System/SystemInventory/Widgets/Storage/WB_Storage.SlotsWidgets` (`self.WB Storage`)) Index)))

(fn `AddItem`
  (params (ItemClass :type "/Game/System/SystemInventory/Blueprints/ItemClasses/items/bp_MasterItem Class Reference") (Amount :type Integer))
  (returns (`Success?` :type Boolean) (Rest :type Integer))
  (locals (Local_FoundIndex :type Integer :default 0) (Local_ItemClass :type "/Game/System/SystemInventory/Blueprints/ItemClasses/items/bp_MasterItem Class Reference") (Local_Amount :type Integer))
  (bind _local_amount (`local.Local_Amount`))
  (bind _slots (`self.Slots`))
  (bind _returnvalue (+ (`.Amount_5_A24D12CF4AB976D01465479176E6C97A` (break `/Game/System/SystemInventory/Blueprints/Structures/s_InventorySlot` (`|GetArrayItem` (`self.Slots`) (`local.Local_FoundIndex`)))) (`local.Local_Amount`)))
  (set `local.Local_ItemClass` ItemClass)
  (set `local.Local_Amount` Amount)
  (if (`.CanBeStacked_16_2123A32242EADFDB737F42A1F9914535` (break `/Game/System/SystemInventory/Blueprints/Structures/S_ItemInfo` (defaults `Object` ItemClass)))
    (bind (_success_ _index) (`self.SearchFreeStack` (`local.Local_ItemClass`)))
    (if _success_
      (set `local.Local_FoundIndex` _index)
      (if (> _returnvalue (`self.MaxStackSize`))
        (set `local.Local_Amount` (- _returnvalue (`self.MaxStackSize`)))
        (`KismetArrayLibrary.Array_Set` _slots (`local.Local_FoundIndex`) (make `/Game/System/SystemInventory/Blueprints/Structures/s_InventorySlot` (`local.Local_ItemClass`) (`self.MaxStackSize`)))
        (`self.UpdateSlotsAtIndex` (`local.Local_FoundIndex`))
        (bind (_success__2 _rest) (`self.AddItem` (`local.Local_ItemClass`) (`local.Local_Amount`)))
        (return _success__2 _rest)
        (else
          (`KismetArrayLibrary.Array_Set` _slots (`local.Local_FoundIndex`) (make `/Game/System/SystemInventory/Blueprints/Structures/s_InventorySlot` (`local.Local_ItemClass`) _returnvalue))
          (`self.UpdateSlotsAtIndex` (`local.Local_FoundIndex`))
          (return true 0)))
      (else
        (bind (_success__3 _index_2) (`self.SearchEmptySlots`))
        (if _success__3
          (bind _output_get (set `local.Local_FoundIndex` _index_2))
          (if (> (`local.Local_Amount`) (`self.MaxStackSize`))
            (`KismetArrayLibrary.Array_Set` (`self.Slots`) _output_get (make `/Game/System/SystemInventory/Blueprints/Structures/s_InventorySlot` (`local.Local_ItemClass`) (`self.MaxStackSize`)))
            (`self.UpdateSlotsAtIndex` (`local.Local_FoundIndex`))
            (bind (_success__4 _rest_2) (`self.AddItem` (`local.Local_ItemClass`) (- (`local.Local_Amount`) (`self.MaxStackSize`))))
            (return true _rest_2)
            (else
              (`KismetArrayLibrary.Array_Set` (`self.Slots`) (`local.Local_FoundIndex`) (make `/Game/System/SystemInventory/Blueprints/Structures/s_InventorySlot` (`local.Local_ItemClass`) (`local.Local_Amount`)))
              (`self.UpdateSlotsAtIndex` (`local.Local_FoundIndex`))
              (return true 0)))
          (else
            (return false (`local.Local_Amount`))))))
    (else
      ;[1 1 1] логика для одиночных предметов(не количественных)
      (bind (_success__5 _index_3) (`self.SearchEmptySlots`))
      (if _success__5
        (bind _output_get_2 (set `local.Local_FoundIndex` _index_3))
        (`KismetArrayLibrary.Array_Set` (`self.Slots`) _output_get_2 (make `/Game/System/SystemInventory/Blueprints/Structures/s_InventorySlot` (`local.Local_ItemClass`) 1))
        (`self.UpdateSlotsAtIndex` (`local.Local_FoundIndex`))
        (if (> _local_amount 1)
          (bind (_success__6 _rest_3) (`self.AddItem` (`local.Local_ItemClass`) (- _local_amount 1)))
          (return true _rest_3)
          (else
            (return true 0)))
        (else
          (return false (`local.Local_Amount`)))))))

(fn `AddItemToIndex`
  (params (Index :type Integer) (Amount :type Integer) (ItemClass :type "/Game/System/SystemInventory/Blueprints/ItemClasses/items/bp_MasterItem Class Reference"))
  (returns (Success :type Boolean))
  (if (and (`self.IsSlotEmpty?` Index) (<= Amount (`self.MaxStackSize`)))
    (`KismetArrayLibrary.Array_Set` (`self.Slots`) Index (make `/Game/System/SystemInventory/Blueprints/Structures/s_InventorySlot` ItemClass Amount))
    (`self.UpdateSlotsAtIndex` Index)
    (return true)
    (else
      (return false))))

(fn `AddToIndex`
  (params (FromIndex :type Integer) (ToIndex :type Integer))
  (returns (`Success?` :type Boolean))
  (locals (LocalFromIndex :type Integer) (LocalToIndex :type Integer) (LocalClass :type "/Game/System/SystemInventory/Blueprints/ItemClasses/items/bp_MasterItem Class Reference"))
  (bind (_output_itemclass _output_amount) (break `/Game/System/SystemInventory/Blueprints/Structures/s_InventorySlot` (`|GetArrayItem` (`self.Slots`) (`local.LocalToIndex`))))
  (bind _output_itemclass_2 (break `/Game/System/SystemInventory/Blueprints/Structures/s_InventorySlot` (`|GetArrayItem` (`self.Slots`) (`local.LocalFromIndex`))))
  (set `local.LocalFromIndex` FromIndex)
  (set `local.LocalToIndex` ToIndex)
  (if (and (== _output_itemclass_2 _output_itemclass) (< _output_amount (`self.MaxStackSize`)) (`.CanBeStacked_16_2123A32242EADFDB737F42A1F9914535` (break `/Game/System/SystemInventory/Blueprints/Structures/S_ItemInfo` (`.ItemInfo` (`self.GetItemInfoAtIndex` (`local.LocalFromIndex`))))))
    (set `local.LocalClass` _output_itemclass_2)
    (if (>= (- (`self.MaxStackSize`) (`self.GetAmountAtIndex` (`local.LocalToIndex`))) (`self.GetAmountAtIndex` (`local.LocalFromIndex`)))
      (`KismetArrayLibrary.Array_Set` (`self.Slots`) (`local.LocalToIndex`) (make `/Game/System/SystemInventory/Blueprints/Structures/s_InventorySlot` (`local.LocalClass`) (+ (`self.GetAmountAtIndex` (`local.LocalFromIndex`)) (`self.GetAmountAtIndex` (`local.LocalToIndex`)))))
      (`KismetArrayLibrary.Array_Set` (`self.Slots`) (`local.LocalFromIndex`) (make `/Game/System/SystemInventory/Blueprints/Structures/s_InventorySlot` null))
      (else
        (`KismetArrayLibrary.Array_Set` (`self.Slots`) (`local.LocalFromIndex`) (make `/Game/System/SystemInventory/Blueprints/Structures/s_InventorySlot` (`local.LocalClass`) (- (`self.GetAmountAtIndex` (`local.LocalFromIndex`)) (- (`self.MaxStackSize`) (`self.GetAmountAtIndex` (`local.LocalToIndex`))))))
        (`KismetArrayLibrary.Array_Set` (`self.Slots`) (`local.LocalToIndex`) (make `/Game/System/SystemInventory/Blueprints/Structures/s_InventorySlot` (`local.LocalClass`) (`self.MaxStackSize`)))))
    (`self.UpdateSlotsAtIndex` (`local.LocalFromIndex`))
    (`self.UpdateSlotsAtIndex` (`local.LocalToIndex`))
    (return true)
    (else
      (return false))))

(fn `GetAmountAtIndex`
  (params (Index :type Integer))
  (returns (Amount :type Integer))
  (return (`.Amount_5_A24D12CF4AB976D01465479176E6C97A` (break `/Game/System/SystemInventory/Blueprints/Structures/s_InventorySlot` (`|GetArrayItem` (`self.Slots`) Index)))))

(fn `GetItemInfoAtIndex`
  (params (index :type Integer))
  (returns (`EmptySlot?` :type Boolean) (ItemInfo :type "/Game/System/SystemInventory/Blueprints/Structures/S_ItemInfo Structure") (Amount :type Integer))
  (bind (_itemclass _amount) (break `/Game/System/SystemInventory/Blueprints/Structures/s_InventorySlot` (`|GetArrayItem` (`self.Slots`) index)))
  (if (`KismetSystemLibrary.IsValidClass` _itemclass)
    (return false (defaults `Object` _itemclass) _amount)
    (else
      (return true (struct) 0))))

(fn `IncreaseAmountAtIndex`
  (params (Index :type Integer) (Amount :type Integer))
  (returns (`Success?` :type Boolean))
  (bind _slots (`self.Slots`))
  (bind (_output_itemclass _output_amount) (break `/Game/System/SystemInventory/Blueprints/Structures/s_InventorySlot` (`|GetArrayItem` _slots Index)))
  (if (and (not (`self.IsSlotEmpty?` Index)) (<= (+ (`self.GetAmountAtIndex` Index) Amount) (`self.MaxStackSize`)))
    (`KismetArrayLibrary.Array_Set` _slots Index (make `/Game/System/SystemInventory/Blueprints/Structures/s_InventorySlot` _output_itemclass (+ _output_amount Amount)))
    (`self.UpdateSlotsAtIndex` Index)
    (return true)
    (else
      (return true))))

(fn `IsSlotEmpty?`
  (params (Index :type Integer))
  (returns (Empty :type Boolean))
  (return (not (`KismetSystemLibrary.IsValidClass` (`.ItemClass_8_6E81B15240E18385B7F49EAFAFC4F40B` (break `/Game/System/SystemInventory/Blueprints/Structures/s_InventorySlot` (`|GetArrayItem` (`self.Slots`) Index)))))))

(fn `MoveFromInvToStorageIndex`
  (params (Inventory :type "/Game/System/SystemInventory/Blueprints/BP_Inventory Object Reference") (InventoryIndex :type Integer) (StorageIndex :type Integer))
  (returns (`Success?` :type Boolean))
  (locals (LocalInventory :type "/Game/System/SystemInventory/Blueprints/BP_Inventory Object Reference") (Local_InvIndex :type Integer) (Local_StorIndex :type Integer) (LocalAmount :type Integer :default 0))
  (bind _localinventory (`local.LocalInventory`))
  (bind _amount (`/Game/System/SystemInventory/Blueprints/BP_Inventory.GetAmountAtIndex` (`local.LocalInventory`) (`local.Local_InvIndex`)))
  (bind _returnvalue (- (`self.MaxStackSize`) (`self.GetAmountAtIndex` (`local.Local_StorIndex`))))
  (set `local.LocalInventory` Inventory)
  (set `local.Local_InvIndex` InventoryIndex)
  (bind _output_get (set `local.Local_StorIndex` StorageIndex))
  (if (`self.IsSlotEmpty?` _output_get)
    (set `local.LocalAmount` (`/Game/System/SystemInventory/Blueprints/BP_Inventory.GetAmountAtIndex` _localinventory (`local.Local_InvIndex`)))
    (bind _success (`self.AddItemToIndex` (`local.Local_StorIndex`) (`local.LocalAmount`) (`.ItemClass_8_6E81B15240E18385B7F49EAFAFC4F40B` (break `/Game/System/SystemInventory/Blueprints/Structures/s_InventorySlot` (`|GetArrayItem` (`/Game/System/SystemInventory/Blueprints/BP_Inventory.Slots` _localinventory) (`local.Local_InvIndex`))))))
    (if _success
      (`/Game/System/SystemInventory/Blueprints/BP_Inventory.RemoveItemAtIndex` (`local.LocalInventory`) (`local.Local_InvIndex`) (`local.LocalAmount`) false)
      (return true)
      (else
        (return false)))
    (elif (and (== (`.ItemClass_8_6E81B15240E18385B7F49EAFAFC4F40B` (break `/Game/System/SystemInventory/Blueprints/Structures/s_InventorySlot` (`|GetArrayItem` (`self.Slots`) (`local.Local_StorIndex`)))) (`.ItemClass_8_6E81B15240E18385B7F49EAFAFC4F40B` (break `/Game/System/SystemInventory/Blueprints/Structures/s_InventorySlot` (`|GetArrayItem` (`/Game/System/SystemInventory/Blueprints/BP_Inventory.Slots` (`local.LocalInventory`)) (`local.Local_InvIndex`))))) (`.CanBeStacked_16_2123A32242EADFDB737F42A1F9914535` (break `/Game/System/SystemInventory/Blueprints/Structures/S_ItemInfo` (`.ItemInfo` (`self.GetItemInfoAtIndex` (`local.Local_StorIndex`))))) (< (`self.GetAmountAtIndex` (`local.Local_StorIndex`)) (`self.MaxStackSize`)))
      (set `local.LocalAmount` (`KismetMathLibrary.SelectInt` _amount _returnvalue (> _amount _returnvalue)))
      (bind _success_ (`self.IncreaseAmountAtIndex` (`local.Local_StorIndex`) (`local.LocalAmount`)))
      (if _success_
        (`/Game/System/SystemInventory/Blueprints/BP_Inventory.RemoveItemAtIndex` (`local.LocalInventory`) (`local.Local_InvIndex`) (`local.LocalAmount`) false)
        (return true)
        (else
          (return false)))
      (else
        (return false)))))

(fn `RemoveItemAtIndex`
  (params (Index :type Integer) (Amount :type Integer) (IsSpawn :type Boolean))
  (returns (Success :type Boolean))
  (locals (LocalIndex :type Integer) (LocalAmount :type Integer) (LocalSpawnItem :type "/Game/System/SystemInventory/Blueprints/Structures/s_InventorySlot Structure"))
  (bind _localindex (`local.LocalIndex`))
  (bind _slots (`self.Slots`))
  (bind (_output_itemclass _output_amount) (break `/Game/System/SystemInventory/Blueprints/Structures/s_InventorySlot` (`|GetArrayItem` _slots _localindex)))
  (set `local.LocalIndex` Index)
  (set `local.LocalAmount` Amount)
  (if (and (not (`self.IsSlotEmpty?` (`local.LocalIndex`))) (> (`local.LocalAmount`) 0))
    (set `local.LocalSpawnItem` (`|GetArrayItem` (`self.Slots`) (`local.LocalIndex`)))
    (if (>= (`local.LocalAmount`) (`self.GetAmountAtIndex` (`local.LocalIndex`)))
      (`KismetArrayLibrary.Array_Set` (`self.Slots`) (`local.LocalIndex`) (make `/Game/System/SystemInventory/Blueprints/Structures/s_InventorySlot` null))
      (`self.UpdateSlotsAtIndex` (`local.LocalIndex`))
      (else
        (`KismetArrayLibrary.Array_Set` _slots _localindex (make `/Game/System/SystemInventory/Blueprints/Structures/s_InventorySlot` _output_itemclass (- _output_amount (`local.LocalAmount`))))
        (`self.UpdateSlotsAtIndex` (`local.LocalIndex`))))
    (if IsSpawn
      (`self.SpawnItemClassInWorld` (`.ItemClass_8_6E81B15240E18385B7F49EAFAFC4F40B` (break `/Game/System/SystemInventory/Blueprints/Structures/s_InventorySlot` (`local.LocalSpawnItem`))) (`local.LocalAmount`))
      (return true)
      (else
        (return true)))
    (else
      (return false))))

(fn `SearchEmptySlots`
  (returns (`Success?` :type Boolean) (Index :type Integer))
  (locals (Local_Bool :type Boolean) (Local_Index :type Integer))
  (for (_array_element _array_index) (`self.Slots`)
    (if (not (`KismetSystemLibrary.IsValidClass` (`.ItemClass_8_6E81B15240E18385B7F49EAFAFC4F40B` (break `/Game/System/SystemInventory/Blueprints/Structures/s_InventorySlot` _array_element))))
      (set `local.Local_Bool` true)
      (set `local.Local_Index` _array_index)
      (break)))
  (return (`local.Local_Bool`) (`local.Local_Index`)))

(fn `SearchFreeStack`
  (params (ItemClass :type "/Game/System/SystemInventory/Blueprints/ItemClasses/items/bp_MasterItem Class Reference"))
  (returns (`Success?` :type Boolean) (Index :type Integer))
  (locals (Local_Bool :type Boolean) (Local_Index :type Integer))
  (for (_array_element _array_index) (`self.Slots`)
    (bind (_itemclass _amount) (break `/Game/System/SystemInventory/Blueprints/Structures/s_InventorySlot` _array_element))
    (if (`KismetSystemLibrary.IsValidClass` _itemclass)
      (if (and (== _itemclass ItemClass) (< _amount (`self.MaxStackSize`)))
        (set `local.Local_Bool` true)
        (set `local.Local_Index` _array_index)
        (break))))
  (return (`local.Local_Bool`) (`local.Local_Index`)))

(fn `SpawnItemClassInWorld`
  (params (ItemClass :type "/Game/System/SystemInventory/Blueprints/ItemClasses/items/bp_MasterItem Class Reference") (AMount :type Integer))
  (locals (LocalRotation :type Integer) (LocalItem :type "/Game/System/SystemInventory/Blueprints/ItemClasses/items/bp_MasterItem Class Reference") (LocalAmount :type Integer) (LocalTrowAway :type Boolean))
  (bind _capsulecomponent (`Character.CapsuleComponent` (`self.TopDownCharRef`)))
  (bind _capsulecomponent_2 (`Character.CapsuleComponent` (`self.TopDownCharRef`)))
  (bind _returnvalue (`SceneComponent.K2_GetComponentLocation` _capsulecomponent))
  (set `local.LocalItem` ItemClass)
  (set `local.LocalAmount` AMount)
  (for _ (range 361)
    (bind _output_get (set `local.LocalRotation` (+ (`local.LocalRotation`) 15)))
    (`SceneComponent.K2_SetWorldRotation` _capsulecomponent (`KismetMathLibrary.MakeRotator` (.roll (`SceneComponent.K2_GetComponentRotation` _capsulecomponent)) (.pitch (`SceneComponent.K2_GetComponentRotation` _capsulecomponent)) (+ (.yaw (`SceneComponent.K2_GetComponentRotation` _capsulecomponent)) (`KismetMathLibrary.Conv_IntToDouble` _output_get))) false false)
    (bind (_outhit _returnvalue_2) (`KismetSystemLibrary.LineTraceSingle` :`Start` _returnvalue :`End` (+ _returnvalue (* (`SceneComponent.GetForwardVector` _capsulecomponent) (`self.DistanceSpawn`))) :`TraceChannel` "TraceTypeQuery1" :`DrawDebugType` "ForDuration"))
    (if (not _returnvalue_2)
      (`|SpawnActorFromClass` "/Game/System/SystemInventory/Blueprints/ItemClasses/BP_PickUpActor.BP_PickUpActor_C" (`KismetMathLibrary.MakeTransform` (+ (`SceneComponent.K2_GetComponentLocation` _capsulecomponent_2) (* (`SceneComponent.GetForwardVector` _capsulecomponent_2) (`self.DistanceSpawn`))) (.rotation (`.WorldView_33_78C9651C41616FEB80780BB0897ABF15` (break `/Game/System/SystemInventory/Blueprints/Structures/S_ItemInfo` (defaults `Object` (`local.LocalItem`))))) (.scale (`.WorldView_33_78C9651C41616FEB80780BB0897ABF15` (break `/Game/System/SystemInventory/Blueprints/Structures/S_ItemInfo` (defaults `Object` (`local.LocalItem`)))))) "Undefined" "OverrideRootScale" null (`local.LocalItem`) (`local.LocalAmount`) 0 null)
      (set `local.LocalTrowAway` true)
      (break)))
  (if (`local.LocalTrowAway`)
    (return)
    (else
      (`|SpawnActorFromClass` "/Game/System/SystemInventory/Blueprints/ItemClasses/BP_PickUpActor.BP_PickUpActor_C" (`KismetMathLibrary.MakeTransform` (`SceneComponent.K2_GetComponentLocation` (`Character.CapsuleComponent` (`self.TopDownCharRef`))) (.rotation (`.WorldView_33_78C9651C41616FEB80780BB0897ABF15` (break `/Game/System/SystemInventory/Blueprints/Structures/S_ItemInfo` (defaults `Object` (`local.LocalItem`))))) (.scale (`.WorldView_33_78C9651C41616FEB80780BB0897ABF15` (break `/Game/System/SystemInventory/Blueprints/Structures/S_ItemInfo` (defaults `Object` (`local.LocalItem`)))))) "Undefined" "OverrideRootScale" null (`local.LocalItem`) (`local.LocalAmount`) 0 null)
      (return))))

(fn `SwapSlots`
  (params (Index1 :type Integer) (Index2 :type Integer))
  (returns (`Success?` :type Boolean))
  (locals (LocalIndex1 :type Integer) (LocalIndex2 :type Integer) (LocalSlot2 :type "/Game/System/SystemInventory/Blueprints/Structures/s_InventorySlot Structure"))
  (bind _slots (`self.Slots`))
  (bind _returnvalue (`KismetArrayLibrary.Array_LastIndex` (`self.Slots`)))
  (set `local.LocalIndex1` Index1)
  (set `local.LocalIndex2` Index2)
  (if (or (> (`local.LocalIndex1`) _returnvalue) (> (`local.LocalIndex2`) _returnvalue))
    (return false)
    (else
      (set `local.LocalSlot2` (`|GetArrayItem` (`self.Slots`) (`local.LocalIndex2`)))
      (`KismetArrayLibrary.Array_Set` _slots (`local.LocalIndex2`) (`|GetArrayItem` _slots (`local.LocalIndex1`)))
      (`KismetArrayLibrary.Array_Set` (`self.Slots`) (`local.LocalIndex1`) (`local.LocalSlot2`))
      (`self.UpdateSlotsAtIndex` (`local.LocalIndex1`))
      (`self.UpdateSlotsAtIndex` (`local.LocalIndex2`))
      (return true))))

(fn `UserConstructionScript`)

(fn `VisibilityStorage`
  (params (Show :type Boolean))
  (bind _wb_storage (`self.WB Storage`))
  (bind _inventoryref (`/Game/Character/BP_character.InventoryRef` (`self.TopDownCharRef`)))
  (if Show
    (`Widget.SetVisibility` _wb_storage "Visible")
    (set `/Game/System/SystemInventory/Blueprints/BP_Inventory.StorageOpen` true _inventoryref)
    (else
      (`Widget.SetVisibility` _wb_storage "Hidden")
      (set `/Game/System/SystemInventory/Blueprints/BP_Inventory.StorageOpen` false _inventoryref)))
  (return))