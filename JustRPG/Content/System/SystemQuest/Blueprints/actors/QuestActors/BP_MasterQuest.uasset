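; BP_MasterQuest is the base quest actor that tracks one quest's active, completed and failed subgoals, description and state.
; CompleteSubGoal records results, queues following goals by index or ends the quest through QuestManager.
; AddGoalForIndex recursively auto-completes goals whose target class is already in the character's obtained objects, otherwise creating subgoal widgets.
; It updates quest and journal widgets directly, with empty OnGoalCompleted and OnGoalFailed hooks.
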(event `OnQuestCancel`
  (`self.RemoveWidget`)
  (`/Game/System/SystemQuest/Blueprints/actors/BP_QuestManager.CancelQuest` (`self.QuestManager`) self))

(event `OnGoalCompleted`
  (params (GoalIndex :type Integer)))

(event `OnGoalFailed`
  (params (GoalIndex :type Integer)))

(fn `Add Sub Goal Widget`
  (params (Index :type Integer) (GoalInfo :type "/Game/System/SystemQuest/Structures/S_GoalInfo Structure"))
  (bind _questwidget (`self.QuestWidget`))
  (bind _returnvalue (`KismetArrayLibrary.Array_Add` (`self.CurrentGoalIndices`) Index))
  (if (> _returnvalue (`KismetArrayLibrary.Array_LastIndex` (`self.CurrentHuntedAmounts`)))
    (`KismetArrayLibrary.Array_Add` (`self.CurrentHuntedAmounts`)))
  (`KismetArrayLibrary.Array_Add` (`self.CurrentGoal`) GoalInfo)
  (bind _returnvalue_2 (`|CreateWidget` "/Game/System/SystemQuest/Widgets/WB_SubGoal.WB_SubGoal_C" null GoalInfo self (`self.QuestWidget`)))
  (`KismetArrayLibrary.Array_Add` (`/Game/System/SystemQuest/Widgets/WB_Quest.SubGoalWidget` _questwidget) _returnvalue_2)
  (`PanelWidget.AddChild` (`/Game/System/SystemQuest/Widgets/WB_Quest.SubGoalBox` _questwidget) null)
  (return))

(fn `AddGoalForIndex`
  (params (Index :type Integer))
  (locals (LocalIndex :type Integer))
  (bind _localindex (`local.LocalIndex`))
  (bind _localindex_2 (`local.LocalIndex`))
  (bind _goal (`self.GoalAtIndex` _localindex_2))
  (bind _output_get (set `local.LocalIndex` Index))
  (if (`self.GoalAlReadyFound` _output_get)
    (`KismetArrayLibrary.Array_Add` (`self.ComplitedSubGoals`) (make `/Game/System/SystemQuest/Structures/S_CompletedGoal` _localindex_2 _goal true))
    (`self.OnGoalCompleted` (`local.LocalIndex`))
    (`self.Update Description` _goal)
    (for _array_element (`.FollowingSubGoalIndices_30_FFBD011444F77F85974AADA021EB7CC0` (break `/Game/System/SystemQuest/Structures/S_GoalInfo` _goal))
      (`self.AddGoalForIndex` _array_element))
    (else
      (`self.Add Sub Goal Widget` _localindex (`self.GoalAtIndex` _localindex))))
  (return))

(fn `CompleteSubGoal`
  (params (SubGoalIndex :type Integer) (Failed :type Boolean))
  (returns (Success :type Boolean))
  (locals (LocalGoalIndex :type Integer) (LocalCompletedSubGoal :type "/Game/System/SystemQuest/Structures/S_GoalInfo Structure") (LocalWidgetIndex :type Integer :default 0) (LocalFail :type Boolean))
  (bind _questwidget (`self.QuestWidget`))
  (bind _localgoalindex (`local.LocalGoalIndex`))
  (bind _currentgoalindices (`self.CurrentGoalIndices`))
  (bind _localgoalindex_2 (`local.LocalGoalIndex`))
  (bind (_type _customgoal _additionalname _amounttohunt _goalclass _goalid _goaltxt _goallocation _useradius _radius _circlecolor _updatequestdescription_ _updatedescription _followingsubgoalindices _failmeansquestfail _completequest) (break `/Game/System/SystemQuest/Structures/S_GoalInfo` (`local.LocalCompletedSubGoal`)))
  (bind (_type_2 _customgoal_2 _additionalname_2 _amounttohunt_2 _goalclass_2 _goalid_2 _goaltxt_2 _goallocation_2 _useradius_2 _radius_2 _circlecolor_2 _updatequestdescription__2 _updatedescription_2) (break `/Game/System/SystemQuest/Structures/S_GoalInfo` (`local.LocalCompletedSubGoal`)))
  (bind _subgoalwidget (`/Game/System/SystemQuest/Widgets/WB_Quest.SubGoalWidget` (`self.QuestWidget`)))
  (set `local.LocalFail` Failed)
  (set `local.LocalGoalIndex` SubGoalIndex)
  (if (`KismetArrayLibrary.Array_Contains` (`self.CurrentGoalIndices`) (`local.LocalGoalIndex`))
    (bind _output_get (set `local.LocalCompletedSubGoal` (`|GetArrayItem` (`.SubGoals_29_CF0D2FD9423203882C03AC892F428479` (break `/Game/System/SystemQuest/Structures/S_QuestInfo` (`self.QuestInfo`))) (`local.LocalGoalIndex`))))
    (`KismetArrayLibrary.Array_Add` (`self.ComplitedSubGoals`) (make `/Game/System/SystemQuest/Structures/S_CompletedGoal` (`local.LocalGoalIndex`) _output_get (not (`local.LocalFail`))))
    (if (and _updatequestdescription__2 (not (`local.LocalFail`)))
      (set `self.CurrentDescription` (`|FormatText` "{Current} {Next}" (`self.CurrentDescription`) _updatedescription_2))
      (if (`self.SelectedInJournal`)
        (`/Game/System/SystemQuest/Widgets/WB_QuestJournal.UpdateDescription` (`/Game/Widgets/WB_MainWidget.WB_QuestJournal` (`/Game/System/SystemQuest/Blueprints/actors/BP_QuestManager.MainWidget` (`self.QuestManager`))))))
    (`KismetArrayLibrary.Array_RemoveItem` (`self.CurrentGoal`) (`local.LocalCompletedSubGoal`))
    (bind _output_get_2 (set `local.LocalWidgetIndex` (`KismetArrayLibrary.Array_Find` _currentgoalindices _localgoalindex_2)))
    (`KismetArrayLibrary.Array_Remove` (`self.CurrentHuntedAmounts`) _output_get_2)
    (`KismetArrayLibrary.Array_RemoveItem` _currentgoalindices _localgoalindex_2)
    ;[1 1 1] выполненые подцели удаляем здесь
    (`Widget.RemoveFromParent` (`|GetArrayItem` _subgoalwidget (`local.LocalWidgetIndex`)))
    (`KismetArrayLibrary.Array_Remove` _subgoalwidget (`local.LocalWidgetIndex`))
    (if (`local.LocalFail`)
      (`self.OnGoalFailed` _localgoalindex)
      (if (`.FailMeansQuestFail_47_3DDD0B0D4C67A7AD71B2EE9ED927232D` (break `/Game/System/SystemQuest/Structures/S_GoalInfo` (`local.LocalCompletedSubGoal`)))
        _
        (else
          (if (`self.SelectedInJournal`) :!label _label
            (`/Game/System/SystemQuest/Widgets/WB_QuestJournal.GenerateSubGoals` (`/Game/Widgets/WB_MainWidget.WB_QuestJournal` (`/Game/System/SystemQuest/Blueprints/actors/BP_QuestManager.MainWidget` (`self.QuestManager`))))
            (else
              (`/Game/System/SystemQuest/Widgets/WB_Quest.UpdateQuest` (`self.QuestWidget`))))
          (if (and (== (`local.LocalGoalIndex`) (`self.SelectedSubGoalIndex`)) (== (`/Game/System/SystemQuest/Blueprints/actors/BP_QuestManager.CurrentQuest` (`self.QuestManager`)) self))
            (`/Game/System/SystemQuest/Widgets/WB_Quest.SelectSubGoal` _questwidget (`|GetArrayItem` (`/Game/System/SystemQuest/Widgets/WB_Quest.SubGoalWidget` _questwidget)))
            (return true)
            (else
              (return true)))))
      (else
        (`self.OnGoalCompleted` _localgoalindex)
        (if _completequest
          _
          (else
            ;[1 1 1] добавляем новые подцели
            (for _array_element _followingsubgoalindices
              (`self.AddGoalForIndex` _array_element))
            (goto _label)))))
    (for _array_element_2 (`self.CurrentGoalIndices`)
      (`KismetArrayLibrary.Array_Add` (`self.ComplitedSubGoals`) (make `/Game/System/SystemQuest/Structures/S_CompletedGoal` _array_element_2 (`self.GoalAtIndex` _array_element_2))))
    (`KismetArrayLibrary.Array_Clear` (`self.CurrentGoalIndices`))
    (`KismetArrayLibrary.Array_Clear` (`self.CurrentHuntedAmounts`))
    (`KismetArrayLibrary.Array_Clear` (`self.CurrentGoal`))
    (set `self.CurrentState` (select `bool` (`local.LocalFail`) :`false` "NewEnumerator1" :`true` "NewEnumerator2" :!type "/Game/System/SystemQuest/Enums/E_QuestStates Enum"))
    (`self.RemoveWidget`)
    (`/Game/System/SystemQuest/Blueprints/actors/BP_QuestManager.EndQuest` (`self.QuestManager`) self)
    (return true)
    (else
      (return false))))

(fn `GoalAlReadyFound`
  (params (GoalIndex :type Integer))
  (returns (Out :type Boolean))
  (locals (LocalBool :type Boolean))
  (bind (_type _customgoal _additionalname _amounttohunt _goalclass) (break `/Game/System/SystemQuest/Structures/S_GoalInfo` (`self.GoalAtIndex` GoalIndex)))
  (if (`|EnumEquality` _type "NewEnumerator2")
    (for _array_element (`/Game/Character/BP_character.ObtainedObj` (`/Game/System/SystemQuest/Blueprints/actors/BP_QuestManager.Character` (`self.QuestManager`)))
      (if (== _array_element _goalclass)
        (set `local.LocalBool` true)
        (break)))
    (return (`local.LocalBool`))
    (else
      (return false))))

(fn `GoalAtIndex`
  (params (Index :type Integer))
  (returns (Goal :type "/Game/System/SystemQuest/Structures/S_GoalInfo Structure"))
  ;[1 1 1] выдал ошибку
  (return (`|GetArrayItem` (`.SubGoals_29_CF0D2FD9423203882C03AC892F428479` (break `/Game/System/SystemQuest/Structures/S_QuestInfo` (`self.QuestInfo`))) Index)))

(fn `GoToNextSubGoals`
  (returns (`Success?` :type Boolean))
  (locals (LocalNextIndex :type Integer :default 0))
  (bind _currentgoalindices (`self.CurrentGoalIndices`))
  (bind _returnvalue (+ (`.MaxValue` (`KismetMathLibrary.MaxOfIntArray` (`self.CurrentGoalIndices`))) 1))
  (if (<= _returnvalue (`KismetArrayLibrary.Array_Length` (`.SubGoals_29_CF0D2FD9423203882C03AC892F428479` (break `/Game/System/SystemQuest/Structures/S_QuestInfo` (`self.QuestInfo`)))))
    (bind _output_get (set `local.LocalNextIndex` _returnvalue))
    (`KismetArrayLibrary.Array_Clear` _currentgoalindices)
    (`KismetArrayLibrary.Array_Add` _currentgoalindices _output_get)
    (`self.UpdateSubGoals`)
    (return true)
    (else
      (return false))))

(fn `RemoveWidget`
  (bind _listentrywidget (`self.ListEntryWidget`))
  (bind _mainwidget (`/Game/System/SystemQuest/Blueprints/actors/BP_QuestManager.MainWidget` (`self.QuestManager`)))
  (`KismetArrayLibrary.Array_RemoveItem` (`/Game/Widgets/WB_MainWidget.QuestWidget` _mainwidget) (`self.QuestWidget`))
  (`KismetArrayLibrary.Array_RemoveItem` (`/Game/System/SystemQuest/Widgets/WB_QuestJournal.AllQuestEntry` (`/Game/Widgets/WB_MainWidget.WB_QuestJournal` _mainwidget)) _listentrywidget)
  (`Widget.RemoveFromParent` _listentrywidget)
  (`Widget.RemoveFromParent` (`self.QuestWidget`)))

(fn `SelectedInJournal`
  (returns (Out :type Boolean))
  (bind _selectedquest (`/Game/System/SystemQuest/Widgets/WB_QuestJournal.SelectedQuest` (`/Game/Widgets/WB_MainWidget.WB_QuestJournal` (`/Game/System/SystemQuest/Blueprints/actors/BP_QuestManager.MainWidget` (`self.QuestManager`)))))
  (return (and (`KismetSystemLibrary.IsValid` _selectedquest) (== _selectedquest self))))

(fn `SetupStartingGoals`
  (`KismetArrayLibrary.Array_Clear` (`self.CurrentGoalIndices`))
  (set `self.CurrentDescription` (`.Description_9_6EAA31F949FBF19869CC0B9E43508742` (break `/Game/System/SystemQuest/Structures/S_QuestInfo` (`self.QuestInfo`))))
  (for _array_element (`self.StartingSubGoalIndices`)
    (`self.AddGoalForIndex` _array_element))
  (`KismetArrayLibrary.Array_Resize` (`self.CurrentHuntedAmounts`) (`KismetArrayLibrary.Array_Length` (`self.CurrentGoalIndices`)))
  (`self.UpdateSubGoals`)
  (return))

(fn `Update Description`
  (params (GoalInfo :type "/Game/System/SystemQuest/Structures/S_GoalInfo Structure"))
  (bind (_type _customgoal _additionalname _amounttohunt _goalclass _goalid _goaltxt _goallocation _useradius _radius _circlecolor _updatequestdescription_ _updatedescription) (break `/Game/System/SystemQuest/Structures/S_GoalInfo` GoalInfo))
  (if _updatequestdescription_
    (set `self.CurrentDescription` (`|FormatText` "{Current} {Next}" (`self.CurrentDescription`) _updatedescription))
    (if (`self.SelectedInJournal`)
      (`/Game/System/SystemQuest/Widgets/WB_QuestJournal.UpdateDescription` (`/Game/Widgets/WB_MainWidget.WB_QuestJournal` (`/Game/System/SystemQuest/Blueprints/actors/BP_QuestManager.MainWidget` (`self.QuestManager`))))))
  (return))

(fn `UpdateSubGoals`
  (`KismetArrayLibrary.Array_Clear` (`self.CurrentGoal`))
  (for _array_element (`self.CurrentGoalIndices`)
    (`KismetArrayLibrary.Array_Add` (`self.CurrentGoal`) (`|GetArrayItem` (`.SubGoals_29_CF0D2FD9423203882C03AC892F428479` (break `/Game/System/SystemQuest/Structures/S_QuestInfo` (`self.QuestInfo`))) _array_element)))
  (return))

(fn `UserConstructionScript`)