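; Quest manager actor that spawns quest actors, tracks current, completed and failed quests, and keeps the journal and quest list in sync.
; NPC talk, item found and enemy kill events advance matching subgoals, deferring quest-completing ones until iteration ends.
; The selected subgoal can spawn a goal marker driving distance text and a minimap arrow.
; Ending a completed quest grants experience, regional prestige and coins; cancelling notifies the client NPC.
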(event `OnTalkToNPC`
  (params (NPCClass :type "/Game/Character/MasterNPC Class Reference") (NPC_ID :type Integer))
  ;[1 1 1] квест, поговорить с NPC
  (`KismetArrayLibrary.Array_Clear` (`self.IndicesToCompleteLater`))
  (for _array_element (`self.CurrentQuestActors`)
    (for (_array_element_2 _array_index) (`/Game/System/SystemQuest/Blueprints/actors/QuestActors/BP_MasterQuest.CurrentGoal` _array_element)
      (bind (_type _customgoal _additionalname _amounttohunt _goalclass _goalid _goaltxt _goallocation _useradius _radius _circlecolor _updatequestdescription_ _updatedescription _followingsubgoalindices _failmeansquestfail _completequest) (break `/Game/System/SystemQuest/Structures/S_GoalInfo` _array_element_2))
      (if (`|EnumEquality` _type "NewEnumerator3")
        (if _completequest
          (bind _output (`|GetArrayItem` (`/Game/System/SystemQuest/Blueprints/actors/QuestActors/BP_MasterQuest.CurrentGoalIndices` _array_element) _array_index))
          (`KismetArrayLibrary.Array_Add` (`self.IndicesToCompleteLater`) (make `/Game/System/SystemQuest/Structures/S_IndexToComplete` _array_element _output))
          (else
            (`/Game/System/SystemQuest/Blueprints/actors/QuestActors/BP_MasterQuest.CompleteSubGoal` _array_element _output false))))))
  (`self.Complete Goals`))

(event `OnObjFound`
  (params (FoundObj :type "/Game/System/SystemQuest/Blueprints/actors/Obj/MasterObj Class Reference"))
  ;[1 1 1] квест поиска предметов, выполнен
  (`KismetArrayLibrary.Array_Clear` (`self.IndicesToCompleteLater`))
  (set `self.Found Obj` FoundObj)
  (for _array_element (`self.CurrentQuestActors`)
    (for (_array_element_2 _array_index) (`/Game/System/SystemQuest/Blueprints/actors/QuestActors/BP_MasterQuest.CurrentGoal` _array_element)
      (bind (_type _customgoal _additionalname _amounttohunt _goalclass _goalid _goaltxt _goallocation _useradius _radius _circlecolor _updatequestdescription_ _updatedescription _followingsubgoalindices _failmeansquestfail _completequest) (break `/Game/System/SystemQuest/Structures/S_GoalInfo` _array_element_2))
      (if (and (`|EnumEquality` _type "NewEnumerator2") (== _goalclass (`self.Found Obj`)))
        (if _completequest
          (bind _output (`|GetArrayItem` (`/Game/System/SystemQuest/Blueprints/actors/QuestActors/BP_MasterQuest.CurrentGoalIndices` _array_element) _array_index))
          (`KismetArrayLibrary.Array_Add` (`self.IndicesToCompleteLater`) (make `/Game/System/SystemQuest/Structures/S_IndexToComplete` _array_element _output))
          (else
            (`/Game/System/SystemQuest/Blueprints/actors/QuestActors/BP_MasterQuest.CompleteSubGoal` _array_element _output false))))))
  (`self.Complete Goals`))

(event `OnEnemyKilled`
  (params (Class :type "/Game/Character/Enemy/MasterEnemy Class Reference"))
  ;[1 1 1] квест убийства мобов
  (`KismetArrayLibrary.Array_Clear` (`self.IndicesToCompleteLater`))
  (set `self.KilledEnemy` Class)
  (for _array_element (`self.CurrentQuestActors`)
    (for (_array_element_2 _array_index) (`/Game/System/SystemQuest/Blueprints/actors/QuestActors/BP_MasterQuest.CurrentGoal` _array_element)
      (bind (_type _customgoal _additionalname _amounttohunt _goalclass _goalid _goaltxt _goallocation _useradius _radius _circlecolor _updatequestdescription_ _updatedescription _followingsubgoalindices _failmeansquestfail _completequest) (break `/Game/System/SystemQuest/Structures/S_GoalInfo` _array_element_2))
      (if (and (`|EnumEquality` _type "NewEnumerator1") (== _goalclass (`self.KilledEnemy`)))
        (bind _returnvalue (+ (`|GetArrayItem` (`/Game/System/SystemQuest/Blueprints/actors/QuestActors/BP_MasterQuest.CurrentHuntedAmounts` _array_element) _array_index) 1))
        (if (>= _returnvalue _amounttohunt)
          (if _completequest
            (bind _output (`|GetArrayItem` (`/Game/System/SystemQuest/Blueprints/actors/QuestActors/BP_MasterQuest.CurrentGoalIndices` _array_element) _array_index))
            (`KismetArrayLibrary.Array_Add` (`self.IndicesToCompleteLater`) (make `/Game/System/SystemQuest/Structures/S_IndexToComplete` _array_element _output))
            (else
              (`/Game/System/SystemQuest/Blueprints/actors/QuestActors/BP_MasterQuest.CompleteSubGoal` _array_element _output false)))
          (else
            (`KismetArrayLibrary.Array_Set` (`/Game/System/SystemQuest/Blueprints/actors/QuestActors/BP_MasterQuest.CurrentHuntedAmounts` _array_element) _array_index _returnvalue)
            (`/Game/System/SystemQuest/Widgets/WB_SubGoal.Update` (`|GetArrayItem` (`/Game/System/SystemQuest/Widgets/WB_Quest.SubGoalWidget` (`/Game/System/SystemQuest/Blueprints/actors/QuestActors/BP_MasterQuest.QuestWidget` _array_element)) _array_index))
            (if (`/Game/System/SystemQuest/Blueprints/actors/QuestActors/BP_MasterQuest.SelectedInJournal` _array_element)
              (`/Game/System/SystemQuest/Widgets/WB_QuestJournal.GenerateSubGoals` (`/Game/Widgets/WB_MainWidget.WB_QuestJournal` (`self.MainWidget`)))))))))
  (`self.Complete Goals`))

(event `OnswitchSubQuest`
  (bind _currentquest (`self.CurrentQuest`))
  (bind _mainwidget (`self.MainWidget`))
  (`/Engine/EditorBlueprintResources/StandardMacros.IsValid` (`self.CurrentGoalActor`)
    (:`Is Valid`
      (`self.K2_DestroyActor` (`self.CurrentGoalActor`)))
    (:`Is Not Valid`
      _))
  (bind _output_get (set `self.CurrentSubGoal` (`|GetArrayItem` (`.SubGoals_29_CF0D2FD9423203882C03AC892F428479` (break `/Game/System/SystemQuest/Structures/S_QuestInfo` (`/Game/System/SystemQuest/Blueprints/actors/QuestActors/BP_MasterQuest.QuestInfo` _currentquest))) (`/Game/System/SystemQuest/Blueprints/actors/QuestActors/BP_MasterQuest.SelectedSubGoalIndex` _currentquest))))
  (bind (_type _customgoal _additionalname _amounttohunt _goalclass _goalid _goaltxt _goallocation _useradius _radius _circlecolor) (break `/Game/System/SystemQuest/Structures/S_GoalInfo` _output_get))
  (bind (_haslocation_ _location) (break `/Game/System/SystemQuest/Structures/S_GoalLocation` _goallocation))
  (if _haslocation_
    (bind _returnvalue (`|SpawnActorFromClass` "/Game/System/SystemQuest/Blueprints/actors/BP_GoalActor.BP_GoalActor_C" (`KismetMathLibrary.MakeTransform` _location) "AlwaysSpawn" "OverrideRootScale" null _useradius _radius _circlecolor null))
    (set `self.CurrentGoalActor` _returnvalue)
    (bind _output_get_2 (set `self.CurrentDistance` (`self.DistanceToGoal`)))
    (`TextBlock.SetText` (`/Game/Widgets/WB_MainWidget.DistanceTxt` (`self.MainWidget`)) (`KismetTextLibrary.Conv_IntToText` _output_get_2 false false))
    (`self.UpdateDirectionArrow`)
    (`Widget.SetVisibility` (`/Game/Widgets/WB_MainWidget.DistanceBorder` _mainwidget) "HitTestInvisible")
    (`Widget.SetVisibility` (`/Game/System/SystemQuest/MiniMap/WB_MiniMap.DirectionArrow` (`/Game/Widgets/WB_MainWidget.WB_MiniMap` _mainwidget)) (select `bool` (> (`self.CurrentDistance`) (`self.ShowDirectionArrowAmount`)) :`false` "Hidden" :`true` "HitTestInvisible" :!type "ESlateVisibility Enum"))
    (else
      (set `self.CurrentGoalActor` null)
      (`Widget.SetVisibility` (`/Game/Widgets/WB_MainWidget.DistanceBorder` (`self.MainWidget`)) "Hidden")
      (`Widget.SetVisibility` (`/Game/System/SystemQuest/MiniMap/WB_MiniMap.DirectionArrow` (`/Game/Widgets/WB_MainWidget.WB_MiniMap` (`self.MainWidget`))) "Hidden"))))

(event `OnPlayerMove`
  (bind _directionarrow (`/Game/System/SystemQuest/MiniMap/WB_MiniMap.DirectionArrow` (`/Game/Widgets/WB_MainWidget.WB_MiniMap` (`self.MainWidget`))))
  (`/Engine/EditorBlueprintResources/StandardMacros.IsValid` (`self.CurrentGoalActor`)
    (:`Is Valid`
      (bind _output_get (set `self.CurrentDistance` (`self.DistanceToGoal`)))
      (`TextBlock.SetText` (`/Game/Widgets/WB_MainWidget.DistanceTxt` (`self.MainWidget`)) (`KismetTextLibrary.Conv_IntToText` _output_get false false))
      (`/Engine/EditorBlueprintResources/StandardMacros.CompareInt` (`self.CurrentDistance`) (`self.ShowDirectionArrowAmount`)
        (:`>`
          _)
        (:`==`
          _)
        (:`<`
          (`/Engine/EditorBlueprintResources/StandardMacros.DoOnce` false :!label _label
            (:`Completed`
              (`Widget.SetVisibility` _directionarrow "Hidden")
              (goto _label_2 :!via `Reset`)))))
      (`self.UpdateDirectionArrow`)
      (`/Engine/EditorBlueprintResources/StandardMacros.DoOnce` false :!label _label_2
        (:`Completed`
          (`Widget.SetVisibility` _directionarrow "HitTestInvisible")
          (goto _label :!via `Reset`))))))

(event `self.ReceiveBeginPlay`
  (`self.GetAllNPCs`)
  (bind (_found _npc) (`self.FindNPCByID` "/Game/Character/MasterNPC.MasterNPC_C" 1))
  (if _found
    (set `self.ElderNPC` _npc)))

(fn `AddNewQuest`
  (params (QuestClass :type "/Game/System/SystemQuest/Blueprints/actors/QuestActors/BP_MasterQuest Class Reference") (DirectlyStart :type Boolean))
  (returns (Success :type Boolean))
  (locals (LocalQuestClass :type "/Game/System/SystemQuest/Blueprints/actors/QuestActors/BP_MasterQuest Class Reference") (LoacalDirectlyStart :type Boolean) (`Local QuestActor` :type "/Game/System/SystemQuest/Blueprints/actors/QuestActors/BP_MasterQuest Object Reference"))
  (bind _local_questactor (`local.Local QuestActor`))
  (bind _mainwidget (`self.MainWidget`))
  (set `local.LocalQuestClass` QuestClass)
  (set `local.LoacalDirectlyStart` DirectlyStart)
  (if (and (`KismetSystemLibrary.IsValidClass` QuestClass) (not (`KismetArrayLibrary.Array_Contains` (`self.AllQuestClasses`) QuestClass)))
    (`KismetArrayLibrary.Array_Add` (`self.AllQuestClasses`) (`local.LocalQuestClass`))
    (bind _returnvalue (`|SpawnActorFromClass` (`local.LocalQuestClass`) (`KismetMathLibrary.MakeTransform` (0.0 0.0 0.0)) "AlwaysSpawn" "OverrideRootScale" null self null))
    (bind _output_get (set `local.Local QuestActor` _returnvalue))
    (`KismetArrayLibrary.Array_Add` (`self.CurrentQuestActors`) _output_get)
    (bind _widget (`/Game/Widgets/WB_MainWidget.AddQuestToList` (`self.MainWidget`) _output_get))
    (bind _output_get_2 (set `/Game/System/SystemQuest/Blueprints/actors/QuestActors/BP_MasterQuest.QuestWidget` _widget (`local.Local QuestActor`)))
    (`/Game/System/SystemQuest/Blueprints/actors/QuestActors/BP_MasterQuest.SetupStartingGoals` _output_get)
    (`/Game/System/SystemQuest/Widgets/WB_Quest.UpdateQuest` _output_get_2)
    (`/Game/System/SystemQuest/Widgets/WB_QuestJournal.AddEntry` (`/Game/Widgets/WB_MainWidget.WB_QuestJournal` (`self.MainWidget`)) (`local.Local QuestActor`))
    (if (or (`local.LoacalDirectlyStart`) (>= (`KismetArrayLibrary.Array_Length` (`self.CurrentQuestActors`)) 1))
      (`self.SelectNewQuest` _local_questactor (`|GetArrayItem` (`/Game/System/SystemQuest/Widgets/WB_Quest.SubGoalWidget` (`/Game/System/SystemQuest/Blueprints/actors/QuestActors/BP_MasterQuest.QuestWidget` _local_questactor)))))
    (if (`/Game/Widgets/WB_MainWidget.SlideOut` (`self.MainWidget`))
      (`UserWidget.PlayAnimation` _mainwidget (`/Game/Widgets/WB_MainWidget.SlideOutAnim` _mainwidget) 0.0 1 "Reverse" 1.0 false)
      (set `/Game/Widgets/WB_MainWidget.SlideOut` false _mainwidget)
      (return true)
      (else
        (return true)))
    (else
      (return false))))

(fn `CancelQuest`
  (params (QuestActor :type "/Game/System/SystemQuest/Blueprints/actors/QuestActors/BP_MasterQuest Object Reference"))
  (locals (LocalQuest :type "/Game/System/SystemQuest/Blueprints/actors/QuestActors/BP_MasterQuest Object Reference"))
  (bind _localquest (`local.LocalQuest`))
  (bind _currentgoalactor (`self.CurrentGoalActor`))
  (bind _returnvalue (`GameplayStatics.GetObjectClass` (`local.LocalQuest`)))
  (bind _output (`|GetArrayItem` (`self.CurrentQuestActors`)))
  (bind ((`HasClient_33_BCA85AC94A2835AACBA03EBEBC810CF9` _hasclient) (`ClientClass_35_48CFC25746FE1B2FE306F3AFAF0FF5ED` _clientclass) (`ClientId_37_304CFCF449B26196649A5989107C935A` _clientid)) (break `/Game/System/SystemQuest/Structures/S_QuestInfo` (`/Game/System/SystemQuest/Blueprints/actors/QuestActors/BP_MasterQuest.QuestInfo` _localquest)))
  (bind _output_get (set `local.LocalQuest` QuestActor))
  (`KismetArrayLibrary.Array_RemoveItem` (`self.CurrentQuestActors`) _output_get)
  ;[1 1 1] Скопировано из EndQuest
  (if (== (`local.LocalQuest`) (`self.CurrentQuest`))
    (set `self.CurrentQuest` null)
    (`/Engine/EditorBlueprintResources/StandardMacros.IsValid` _currentgoalactor
      (:`Is Valid`
        (`self.K2_DestroyActor` _currentgoalactor)
        (`Widget.SetVisibility` (`/Game/Widgets/WB_MainWidget.DistanceBorder` (`self.MainWidget`)) "Hidden")
        (`Widget.SetVisibility` (`/Game/System/SystemQuest/MiniMap/WB_MiniMap.DirectionArrow` (`/Game/Widgets/WB_MainWidget.WB_MiniMap` (`self.MainWidget`))) "Hidden"))
      (:`Is Not Valid`
        _))
    (`/Engine/EditorBlueprintResources/StandardMacros.IsValid` _output
      (:`Is Valid`
        (`self.SelectNewQuest` _output (`|GetArrayItem` (`/Game/System/SystemQuest/Widgets/WB_Quest.SubGoalWidget` (`/Game/System/SystemQuest/Blueprints/actors/QuestActors/BP_MasterQuest.QuestWidget` _output)))))
      (:`Is Not Valid`
        _)))
  (if (`/Game/System/SystemQuest/Blueprints/actors/QuestActors/BP_MasterQuest.SelectedInJournal` _localquest)
    (`/Game/System/SystemQuest/Widgets/WB_QuestJournal.OnQuestClicked` (`/Game/Widgets/WB_MainWidget.WB_QuestJournal` (`self.MainWidget`)) null))
  (if _hasclient
    (bind (_found _npc) (`self.FindNPCByID` _clientclass _clientid))
    (if _found
      (`/Game/Character/MasterNPC.OnOwnedQuestCanseled` _npc _returnvalue)))
  (`KismetArrayLibrary.Array_RemoveItem` (`self.AllQuestClasses`) _returnvalue)
  (`self.K2_DestroyActor` (`local.LocalQuest`))
  (return))

(fn `Complete Goals`
  (for _array_element (`self.IndicesToCompleteLater`)
    (`/Game/System/SystemQuest/Blueprints/actors/QuestActors/BP_MasterQuest.CompleteSubGoal` (break `/Game/System/SystemQuest/Structures/S_IndexToComplete` _array_element) (`.Index_5_3CDF6D2B4EB1E987A815539570BA25F5` (break `/Game/System/SystemQuest/Structures/S_IndexToComplete` _array_element)) false)))

(fn `DistanceToGoal`
  (returns (Distance :type Integer))
  (bind (_returnvalue_x _returnvalue_y) (`KismetMathLibrary.BreakVector` (`self.K2_GetActorLocation` (`self.Character`))))
  (bind (_returnvalue_x_2 _returnvalue_y_2) (`KismetMathLibrary.BreakVector` (`self.K2_GetActorLocation` (`self.CurrentGoalActor`))))
  (return (`KismetMathLibrary.Round` (/ (`KismetMathLibrary.VSize` (- (`KismetMathLibrary.MakeVector` _returnvalue_x _returnvalue_y) (`KismetMathLibrary.MakeVector` _returnvalue_x_2 _returnvalue_y_2))) 100.0))))

(fn `EndQuest`
  (params (Quest :type "/Game/System/SystemQuest/Blueprints/actors/QuestActors/BP_MasterQuest Object Reference"))
  (locals (LocalQuest :type "/Game/System/SystemQuest/Blueprints/actors/QuestActors/BP_MasterQuest Object Reference"))
  (bind _localquest (`local.LocalQuest`))
  (bind _character (`self.Character`))
  (bind _localquest_2 (`local.LocalQuest`))
  (bind _currentgoalactor (`self.CurrentGoalActor`))
  (bind _output (`|GetArrayItem` (`self.CurrentQuestActors`)))
  (bind (_name _category _description _region _complitionreward) (break `/Game/System/SystemQuest/Structures/S_QuestInfo` (`/Game/System/SystemQuest/Blueprints/actors/QuestActors/BP_MasterQuest.QuestInfo` (`local.LocalQuest`))))
  (bind _output_get (set `local.LocalQuest` Quest))
  (`KismetArrayLibrary.Array_RemoveItem` (`self.CurrentQuestActors`) _output_get)
  (`KismetArrayLibrary.Array_Add` (select `/Game/System/SystemQuest/Enums/E_QuestStates` (`/Game/System/SystemQuest/Blueprints/actors/QuestActors/BP_MasterQuest.CurrentState` _output_get) :`NewEnumerator0` (`self.CurrentQuestActors`) :`NewEnumerator1` (`self.CompletedQuestActors`) :`NewEnumerator2` (`self.FailedQuestActors`)) _localquest_2)
  (`/Game/System/SystemQuest/Widgets/WB_QuestJournal.AddEntry` (`/Game/Widgets/WB_MainWidget.WB_QuestJournal` (`self.MainWidget`)) _localquest_2)
  (if (== _localquest_2 (`self.CurrentQuest`))
    (set `self.CurrentQuest` null)
    (`/Engine/EditorBlueprintResources/StandardMacros.IsValid` _currentgoalactor
      (:`Is Valid`
        (`self.K2_DestroyActor` _currentgoalactor)
        (`Widget.SetVisibility` (`/Game/Widgets/WB_MainWidget.DistanceBorder` (`self.MainWidget`)) "Hidden")
        (`Widget.SetVisibility` (`/Game/System/SystemQuest/MiniMap/WB_MiniMap.DirectionArrow` (`/Game/Widgets/WB_MainWidget.WB_MiniMap` (`self.MainWidget`))) "Hidden"))
      (:`Is Not Valid`
        _))
    (`/Engine/EditorBlueprintResources/StandardMacros.IsValid` _output
      (:`Is Valid`
        (`self.SelectNewQuest` _output (`|GetArrayItem` (`/Game/System/SystemQuest/Widgets/WB_Quest.SubGoalWidget` (`/Game/System/SystemQuest/Blueprints/actors/QuestActors/BP_MasterQuest.QuestWidget` _output)))))
      (:`Is Not Valid`
        _)))
  (if (`/Game/System/SystemQuest/Blueprints/actors/QuestActors/BP_MasterQuest.SelectedInJournal` _localquest)
    (`/Game/System/SystemQuest/Widgets/WB_QuestJournal.OnQuestClicked` (`/Game/Widgets/WB_MainWidget.WB_QuestJournal` (`self.MainWidget`)) null))
  (if (`|EnumEquality` (`/Game/System/SystemQuest/Blueprints/actors/QuestActors/BP_MasterQuest.CurrentState` _localquest) "NewEnumerator1")
    (`/Game/Character/BP_character.AddExpPoints` _character (break `/Game/System/SystemQuest/Structures/s_QuestReward` _complitionreward))
    (`/Game/Character/BP_character.SetPrestigeByRegion` _character _region (+ (`/Game/Character/BP_character.GetPrestigeByRegion` _character _region) (`.PrestigePoints_6_7C1361924FA8E99DB86B7BA64CCDA12A` (break `/Game/System/SystemQuest/Structures/s_QuestReward` _complitionreward))))
    (`/Game/Character/BP_character.Add Coin` _character (`.Coin_9_ACA60BE14109CF851783299E7F634088` (break `/Game/System/SystemQuest/Structures/s_QuestReward` _complitionreward))))
  (`KismetArrayLibrary.Array_RemoveItem` (`self.AllQuestClasses`) (`GameplayStatics.GetObjectClass` Quest))
  (return))

(fn `FindNPCByID`
  (params (Class :type "/Game/Character/MasterNPC Class Reference") (ID :type Integer))
  (returns (Found :type Boolean) (NPC :type "/Game/Character/MasterNPC Object Reference"))
  (locals (LocalFoundNPC :type "/Game/Character/MasterNPC Object Reference"))
  (for _array_element (`self.OnNPCInWorld`)
    (if (and (== (`GameplayStatics.GetObjectClass` _array_element) Class) (== (`/Game/Character/MasterNPC.NPC_ID` _array_element) ID))
      (set `local.LocalFoundNPC` _array_element)
      (break)))
  (bind _localfoundnpc (`local.LocalFoundNPC`)
    (:`then`
      (return true _localfoundnpc))
    (:`else`
      (return false null))))

(fn `FirstQuestCompleted?`
  (returns (out :type Boolean))
  (locals (Result :type Boolean))
  (for _array_element (`self.CompletedQuestActors`)
    (bind _questinfo_name (break `/Game/System/SystemQuest/Structures/S_QuestInfo` (`/Game/System/SystemQuest/Blueprints/actors/QuestActors/BP_MasterQuest.QuestInfo` _array_element)))
    (if (`KismetTextLibrary.EqualEqual_TextText` _questinfo_name (`KismetTextLibrary.Conv_StringToText` "Первый квест"))
      (set `local.Result` true)
      (break)
      (else
        (set `local.Result` false))))
  (return (`local.Result`)))

(fn `GetAllNPCs`
  (bind _outactors (`GameplayStatics.GetAllActorsOfClass` "/Game/Character/MasterNPC.MasterNPC_C"))
  (set `self.OnNPCInWorld` _outactors)
  (return))

(fn `HasCurrentQuest`
  (params (QuestClass :type "/Game/System/SystemQuest/Blueprints/actors/QuestActors/BP_MasterQuest Class Reference"))
  (returns (Out :type Boolean) (QuestActor :type "/Game/System/SystemQuest/Blueprints/actors/QuestActors/BP_MasterQuest Object Reference"))
  (locals (LocalFoundQuest :type "/Game/System/SystemQuest/Blueprints/actors/QuestActors/BP_MasterQuest Object Reference"))
  (bind _localfoundquest (`local.LocalFoundQuest`))
  (for _array_element (`self.CurrentQuestActors`)
    (if (== (`GameplayStatics.GetObjectClass` _array_element) QuestClass)
      (set `local.LocalFoundQuest` _array_element)
      (break)))
  (`/Engine/EditorBlueprintResources/StandardMacros.IsValid` _localfoundquest
    (:`Is Valid`
      (return true _localfoundquest))
    (:`Is Not Valid`
      (return false null))))

(fn `SelectNewQuest`
  (params (Quest :type "/Game/System/SystemQuest/Blueprints/actors/QuestActors/BP_MasterQuest Object Reference") (`Sub Goal` :type "/Game/System/SystemQuest/Widgets/WB_SubGoal Object Reference"))
  (bind _currentquest (`self.CurrentQuest`))
  (bind _questwidget (`/Game/System/SystemQuest/Blueprints/actors/QuestActors/BP_MasterQuest.QuestWidget` _currentquest))
  (`/Engine/EditorBlueprintResources/StandardMacros.IsValid` _currentquest
    (:`Is Valid`
      (`Widget.SetIsEnabled` (`/Game/System/SystemQuest/Widgets/WB_Quest.QuestName` _questwidget) false)
      (`/Game/System/SystemQuest/Widgets/WB_Quest.SelectSubGoal` _questwidget null))
    (:`Is Not Valid`
      _))
  (bind _output_get (set `self.CurrentQuest` Quest))
  (`/Game/System/SystemQuest/Widgets/WB_Quest.SelectSubGoal` (`/Game/System/SystemQuest/Blueprints/actors/QuestActors/BP_MasterQuest.QuestWidget` _output_get) `Sub Goal`)
  (return))

(fn `UpdateDirectionArrow`
  (bind (_returnvalue_roll _returnvalue_pitch _returnvalue_yaw) (`KismetMathLibrary.BreakRotator` (`KismetMathLibrary.FindLookAtRotation` (`self.K2_GetActorLocation` (`self.Character`)) (`self.K2_GetActorLocation` (`self.CurrentGoalActor`)))))
  (`Widget.SetRenderTransformAngle` (`/Game/System/SystemQuest/MiniMap/WB_MiniMap.DirectionArrow` (`/Game/Widgets/WB_MainWidget.WB_MiniMap` (`self.MainWidget`))) _returnvalue_yaw)
  (return))

(fn `UserConstructionScript`)