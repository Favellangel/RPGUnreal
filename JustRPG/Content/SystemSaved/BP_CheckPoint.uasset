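; BP_CheckPoint is a save point that shows a "Press [q] to save" prompt while the player character is inside its sphere.
; Overlap registers the checkpoint as the character's MarkMap and clears it on exit.
; SaveGame writes player transform, gold, HP and equipped item classes into a new BP_SavedData.
; If the inventory is valid, it calls SaveInventory, saves to slot "1" and prints a confirmation.
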(event `SaveGame`
  (bind _returnvalue (`GameplayStatics.GetPlayerCharacter` 0))
  (bind _topdowncharacter (`self.TopDownCharacter`))
  (bind _inventoryref (`/Game/Character/BP_character.InventoryRef` (`self.TopDownCharacter`)))
  ;[1 1 1] логика Сохранения
  (bind _returnvalue_2 (`GameplayStatics.CreateSaveGameObject` "/Game/SystemSaved/BP_SavedData.BP_SavedData_C"))
  ;;[1 1 1] сохраняем положение игрока
  (set `/Game/SystemSaved/BP_SavedData.Player_Rotation` (`self.K2_GetActorRotation` _returnvalue) _returnvalue_2)
  (set `/Game/SystemSaved/BP_SavedData.Player_Location` (`self.K2_GetActorLocation` _returnvalue) _returnvalue_2)
  (set `/Game/SystemSaved/BP_SavedData.Gold` (`/Game/Character/BP_character.CurrentGold` _topdowncharacter) _returnvalue_2)
  (set `/Game/SystemSaved/BP_SavedData.HP` (`/Game/Character/BP_character.CurrentHP` _topdowncharacter) _returnvalue_2)
  (set `/Game/SystemSaved/BP_SavedData.EquipedWeapon` (`GameplayStatics.GetObjectClass` (`/Game/Character/BP_character.EquippedWeapon` _topdowncharacter)) _returnvalue_2)
  (set `/Game/SystemSaved/BP_SavedData.EquipedClothes` (`GameplayStatics.GetObjectClass` (`/Game/Character/BP_character.EquippedClothes` _topdowncharacter)) _returnvalue_2)
  (`/Engine/EditorBlueprintResources/StandardMacros.IsValid` _inventoryref
    (:`Is Valid`
      (`/Game/System/SystemInventory/Blueprints/BP_Inventory.SaveInventory` _inventoryref)
      (`GameplayStatics.SaveGameToSlot` _returnvalue_2 "1")
      (`/Game/SystemSaved/WBTxtResult.Print` (`/Game/Widgets/WB_MainWidget.WBTxtResult` (`/Game/System/SystemInventory/Blueprints/BP_Inventory.MainWidget` (`/Game/Character/BP_character.InventoryRef` (`self.TopDownCharacter`)))) "Игра Сохранена"))))

(event `self.ReceiveBeginPlay`
  ;[1 1 1] Задаем текст
  (bind _aswb_txt_interaction (cast `/Game/UI/WB_TxtInteraction` (`WidgetComponent.GetUserWidgetObject` (`self.TxtMessage`))))
  (`/Game/UI/WB_TxtInteraction.SetText` _aswb_txt_interaction "Press [q] to save"))

(event `self.SphereCollision.OnComponentBeginOverlap`
  (params (OverlappedComponent :type "PrimitiveComponent Object Reference") (OtherActor :type "Actor Object Reference") (OtherComp :type "PrimitiveComponent Object Reference") (OtherBodyIndex :type Integer) (bFromSweep :type Boolean) (SweepResult :type "HitResult Structure (by ref)"))
  ;[1 1 1] Когда игрок входит в checkPoint
  (bind _asbp_character (cast `/Game/Character/BP_character` OtherActor))
  (bind _output_get (set `self.TopDownCharacter` _asbp_character))
  (set `/Game/Character/BP_character.MarkMap` self _output_get)
  (`SceneComponent.SetVisibility` (`self.TxtMessage`) true false))

(event `self.SphereCollision.OnComponentEndOverlap`
  (params (OverlappedComponent :type "PrimitiveComponent Object Reference") (OtherActor :type "Actor Object Reference") (OtherComp :type "PrimitiveComponent Object Reference") (OtherBodyIndex :type Integer))
  ;[1 1 1] Когда игрок выходит из checkPoint
  (bind _asbp_character (cast `/Game/Character/BP_character` OtherActor))
  (set `/Game/Character/BP_character.MarkMap` null _asbp_character)
  (`SceneComponent.SetVisibility` (`self.TxtMessage`) false false))

(fn `UserConstructionScript`)