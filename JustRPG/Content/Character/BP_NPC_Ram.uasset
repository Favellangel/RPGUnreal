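; BP_NPC_Ram is an NPC character Blueprint that changes its dialogue based on the player's quest progress.
; When talked to, it checks the player's QuestManager for BP_QUestTest1 and whether goal index 2 is among that quest's current goals.
; If so, it shows a Russian line proposing to discuss next steps; otherwise it falls back to the parent's talk behavior.
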(event `self.OnTalkTo`
  (params (Player :type "/Game/Character/BP_character Object Reference"))
  (bind (_out _questactor) (`/Game/System/SystemQuest/Blueprints/actors/BP_QuestManager.HasCurrentQuest` (`/Game/Character/BP_character.QuestManager` Player) "/Game/System/SystemQuest/Blueprints/actors/QuestActors/BP_QUestTest1.BP_QUestTest1_C"))
  (if _out
    (if (`KismetArrayLibrary.Array_Contains` (`/Game/System/SystemQuest/Blueprints/actors/QuestActors/BP_MasterQuest.CurrentGoalIndices` _questactor) 2)
      (`self.ShowMsg` "Отлично, дайвай обсудим что делать дальше")
      (else
        (`parent.OnTalkTo` Player :!label _label)))
    (else
      (goto _label))))

(fn `UserConstructionScript`
  (`parent.UserConstructionScript`))