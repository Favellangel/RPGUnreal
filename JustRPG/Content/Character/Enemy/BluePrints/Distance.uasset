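; Behavior tree task for enemy AI that checks whether the player is within attack range of the controlled pawn.
; It measures the distance between the pawn and the Player blackboard actor and compares it to the AttackRange blackboard value.
; The result is written to the InAttackRange blackboard bool, and the task always finishes successfully.
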(event `self.ReceiveExecuteAI`
  (params (OwnerController :type "AIController Object Reference") (ControlledPawn :type "Pawn Object Reference"))
  (`BTFunctionLibrary.SetBlackboardValueAsBool` (`self.InAttackRange`) (<= (`KismetMathLibrary.VSize` (- (`Actor.K2_GetActorLocation` ControlledPawn) (`Actor.K2_GetActorLocation` (`BTFunctionLibrary.GetBlackboardValueAsActor` (`self.Player`))))) (`BTFunctionLibrary.GetBlackboardValueAsFloat` (`self.AttackRange`))))
  (`self.FinishExecute` true))