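; Behavior tree service that leashes a MasterEnemy to a movement radius around its starting location.
; Each tick it compares the enemy's distance from the blackboard starting point to the radius, skipping the check while a montage plays.
; When exceeded, it sets IsRunningBack and uses AIMoveTo to return home.
; On success, it resets walk speed and clears the running-back and seen-player flags on blackboard and enemy.
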(event `self.ReceiveTickAI`
  (params (OwnerController :type "AIController Object Reference") (ControlledPawn :type "Pawn Object Reference") (DeltaSeconds :type "Float (single-precision)"))
  (bind _enemy (`self.Enemy`))
  (`self.Enemy`
    (:`then`
      _)
    (:`else`
      (bind _asmaster_enemy (cast `/Game/Character/Enemy/MasterEnemy` ControlledPawn))
      (set `self.Enemy` _asmaster_enemy)))
  (if (and (> (`KismetMathLibrary.VSize` (- (`Actor.K2_GetActorLocation` (`self.Enemy`)) (`BTFunctionLibrary.GetBlackboardValueAsVector` (`self.StartingLocation`)))) (`BTFunctionLibrary.GetBlackboardValueAsFloat` (`self.MovamentRadius`))) (not (`/Game/Character/Enemy/MasterEnemy.IsPlayingMontage` (`self.Enemy`))))
    (`BTFunctionLibrary.SetBlackboardValueAsBool` (`self.IsRunningBack`) true)
    (`|AIMoveTo` _enemy _enemy (`BTFunctionLibrary.GetBlackboardValueAsVector` (`self.StartingLocation`)) null
      (:`OnSuccess`
        (set `CharacterMovementComponent.MaxWalkSpeed` 200.0 (`Character.CharacterMovement` _enemy))
        (`BTFunctionLibrary.SetBlackboardValueAsBool` (`self.HasSeenPlayer`))
        (`BTFunctionLibrary.SetBlackboardValueAsBool` (`self.IsRunningBack`))
        (set `/Game/Character/Enemy/MasterEnemy.HasSeenPlayer` false (`self.Enemy`))))))